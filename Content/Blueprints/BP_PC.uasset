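; BP_PC, apparently a player controller, provides mouse edge scrolling by moving CharacterRef along world X and Y.
; Each Tick, four independent checks compare the DPI-scaled cursor position to hard-coded screen margins, so both axes can move together.
; MapRangeClamped ramps speed with depth into each margin, applied as a swept world offset without delta-time scaling.
; CharacterRef is only validity-checked here, never assigned.
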(event EventTick
  (params (DeltaSeconds :type Float%20%28single-precision%29))
  (bind _self self)
  (bind _characterref (Variables|Default|GetCharacterRef))
  (bind _characterref_2 (Variables|Default|GetCharacterRef))
  (bind (_locationx _locationy) (Class|WidgetLayoutLibrary|GetMousePositionScaledbyDPI _self))
  (Variables|Default|GetCharacterRef
    (:then
      (Utilities|FlowControl|Sequence
        (:then_0
          (if (< _locationx 1.5e+02)
            (Transformation|AddActorWorldOffset _characterref_2 (Math|Vector|MakeVector (Math|Float|MapRangeClamped (- 1.5e+02 _locationx) 0.0 1.5e+02 1.0 13.0) 0.0 0.0) true)))
        (:then_1
          (if (> _locationx 1.85e+03)
            (Transformation|AddActorWorldOffset _characterref_2 (Math|Vector|MakeVector (Math|Float|MapRangeClamped (- _locationx 1.85e+03) 0.0 7e+01 -1.0 -13.0) 0.0 0.0) true)))
        (:then_2
          (if (< _locationy 1e+02)
            (Transformation|AddActorWorldOffset _characterref (Math|Vector|MakeVector 0.0 (Math|Float|MapRangeClamped (- 1e+02 _locationy) 0.0 1.5e+02 1.0 13.0) 0.0) true)))
        (:then_3
          (if (> _locationy 1e+03)
            (Transformation|AddActorWorldOffset _characterref (Math|Vector|MakeVector 0.0 (Math|Float|MapRangeClamped (- _locationy 1e+03) 0.0 1.3e+02 -1.0 -13.0) 0.0) true)))))
    (:else)))

(fn ConstructionScript)