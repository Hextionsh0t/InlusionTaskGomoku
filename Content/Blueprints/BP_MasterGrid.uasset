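; BP_MasterGrid builds a rectangular grid board with a surrounding border, sized by GridxCount and GridyCount.
; The construction script lays instanced tiles at 100-unit spacing, using a second instanced mesh for a roughly ten-tile margin outside.
; On BeginPlay it spawns BP_GridPoint actors at tile corners, each receiving a running index and the master AI reference.
; A one-point ring of BP_BlockingPoint actors encloses those points.
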(event EventBeginPlay
  (bind _returnvalue (Transformation|GetActorLocation))
  (bind _gridxcount (Variables|Default|GetgridxCount))
  (bind _gridycount (Variables|Default|GetgridyCount))
  (bind (_x _y _z) (Math|Vector|BreakVector _returnvalue))
  (bind _returnvalue_2 (+ _gridycount 1))
  (bind _returnvalue_3 (+ _gridxcount 1))
  (for _index (range -1 _returnvalue_3)
    (for _index_2 (range -1 _returnvalue_2)
      (if (Math|Boolean|ORBoolean (== _index -1) (== _index _returnvalue_3) (or (== _index_2 -1) (== _index_2 _returnvalue_2)))
        (Game|SpawnActorfromClass "/Game/Blueprints/BP_BlockingPoint.BP_BlockingPoint_C" (Math|Transform|MakeTransform (+ (Math|Vector|MakeVector (- _x 5e+01) (- _y 5e+01) _z) (Math|Vector|MakeVector (* _index 1e+02) (* _index_2 1e+02) 5e+01))) "Undefined" 0 0)
        (else
          (Math|Integer|IncrementInt (Variables|Default|GetGridpointIndex)
            (:%20%20
              (Game|SpawnActorfromClass "/Game/Blueprints/Bp_GridPoint.BP_GridPoint_C" (Math|Transform|MakeTransform (+ (Math|Vector|MakeVector (- _x 5e+01) (- _y 5e+01) _z) (Math|Vector|MakeVector (* _index 1e+02) (* _index_2 1e+02) 5e+01))) "Undefined" 0 (Variables|Default|GetGridpointIndex) (Variables|Default|GetMasterAiRef) 0))))))))

(fn ConstructionScript
  (bind _gridxcount (Variables|Default|GetgridxCount))
  (bind _gridycount (Variables|Default|GetgridyCount))
  (for _index (range 0 (- (Variables|Default|GetgridxCount) 1))
    (for _index_2 (range 0 (- (Variables|Default|GetgridyCount) 1))
      (Class|InstancedStaticMeshComponent|AddInstanceWorldSpace (Variables|Default|GetInstancedStaticMesh) (Math|Transform|MakeTransform (+ (Transformation|GetActorLocation) (Math|Vector|MakeVector (* _index 1e+02) (* _index_2 1e+02) 0.0))))))
  (for _index_3 (range -10 (+ _gridxcount 10))
    (for _index_4 (range -10 (+ _gridycount 10))
      (if (Math|Boolean|ORBoolean (>= _index_4 _gridycount) (<= _index_4 -1) (<= _index_3 -1) (>= _index_3 _gridxcount))
        (Class|InstancedStaticMeshComponent|AddInstanceWorldSpace (Variables|Default|GetInstancedStaticMesh1) (Math|Transform|MakeTransform (+ (Transformation|GetActorLocation) (Math|Vector|MakeVector (* _index_3 1e+02) (* _index_4 1e+02) 0.0))))))))