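; BP_PointEnemyNew is the enemy's placed point in a turn-based grid game, evaluating the lines through it for combo threats.
; On spawn it registers with the player character, plays a drop animation, destroys its grid point and starts tracing.
; AddThreatstoArrays sorts left/right threat levels into local arrays and the master AI's priority combo arrays.
; An enum steps tracing through horizontal, both diagonals and vertical, then hands the turn to the player.
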(event EventAddThreatstoArrays
  (bind _right (Variables|Default|GetRight))
  (bind _masterairef (Variables|Default|GetMasterAIRef))
  (bind _left (Variables|Default|Getleft))
  (bind _countergridindexleft (Variables|Default|GetCounterGridIndexLeft))
  (bind _countergridindexright (Variables|Default|GetCounterGridIndexRight))
  (bind _mediumcomboarray (Variables|/Game/Blueprints/BP_MasterAI.BP_MasterAI_C|GetMediumComboArray _masterairef))
  (bind _instawincombo (Variables|/Game/Blueprints/BP_MasterAI.BP_MasterAI_C|GetInstaWinCombo _masterairef))
  (bind _lowcomboarray (Variables|/Game/Blueprints/BP_MasterAI.BP_MasterAI_C|GetLowComboArray _masterairef))
  (bind _comboarraypriority (Variables|/Game/Blueprints/BP_MasterAI.BP_MasterAI_C|GetComboArrayPriority _masterairef))
  (switch int (Variables|Default|GetLeftThreat)
    (:0
      _)
    (:1
      (Utilities|Array|Add _left (Utilities|Struct|MakeTraceRemoveStruct "NewEnumerator0" _countergridindexleft) :!label _label)
      (Utilities|Array|Add _lowcomboarray _countergridindexleft))
    (:2
      (goto _label))
    (:3
      (goto _label))
    (:4
      (Utilities|Array|Add _left (Utilities|Struct|MakeTraceRemoveStruct "NewEnumerator1" _countergridindexleft))
      (Utilities|Array|Add _mediumcomboarray _countergridindexleft))
    (:5
      (Utilities|Array|Add _left (Utilities|Struct|MakeTraceRemoveStruct "NewEnumerator2" _countergridindexleft))
      (Utilities|Array|Add _comboarraypriority _countergridindexleft))
    (:6
      (Utilities|Array|Add _left (Utilities|Struct|MakeTraceRemoveStruct "NewEnumerator3" _countergridindexleft))
      (Utilities|Array|Add _instawincombo _countergridindexleft)))
  (switch int (Variables|Default|GetRightThreat)
    (:0
      _)
    (:1
      (Utilities|Array|Add _right (Utilities|Struct|MakeTraceRemoveStruct "NewEnumerator0" _countergridindexright) :!label _label_2)
      (Utilities|Array|Add _lowcomboarray _countergridindexright))
    (:2
      (goto _label_2))
    (:3
      (goto _label_2))
    (:4
      (Utilities|Array|Add _right (Utilities|Struct|MakeTraceRemoveStruct "NewEnumerator1" _countergridindexright))
      (Utilities|Array|Add _mediumcomboarray _countergridindexright))
    (:5
      (Utilities|Array|Add _right (Utilities|Struct|MakeTraceRemoveStruct "NewEnumerator2" _countergridindexright))
      (Utilities|Array|Add _comboarraypriority _countergridindexright))
    (:6
      (Utilities|Array|Add _right (Utilities|Struct|MakeTraceRemoveStruct "NewEnumerator3" _countergridindexright))
      (Utilities|Array|Add _instawincombo _countergridindexright)))
  (switch Utilities|FlowControl|Switch|SwitchonTraceEnum (Variables|Default|GetTraceEnum)
    (:NewEnumerator8
      (Variables|Default|SetTraceEnum "NewEnumerator12")
      (CallFunction|TraceUp :!label _label_3))
    (:NewEnumerator13
      (Variables|Default|SetTraceEnum "NewEnumerator14")
      (goto _label_3))
    (:NewEnumerator15
      (Variables|Default|SetTraceEnum "NewEnumerator16")
      (goto _label_3))
    (:NewEnumerator17
      (Default|InitiatePlayerTurn (Variables|Default|GetMasterAIRef)))))

(event EventBeginPlay
  (bind _gridpointref (Variables|Default|GetGridPointRef))
  (bind _staticmesh (Variables|Default|GetStaticMesh))
  (bind _asbp_character (Utilities|Casting|CastToBP_Character (Game|Player|GetPlayerPawn 0)))
  (bind _output_get (Variables|Default|SetCharacterRef _asbp_character))
  (Variables|/Game/Blueprints/BP_Character.BP_Character_C|SetLastPlacedPointEnemy _output_get self)
  (Variables|Default|SetCurrentGridIndex (Variables|/Game/Blueprints/Bp_GridPoint.BP_GridPoint_C|GetGridPointIndex _gridpointref))
  (bind (_direction _newtrack_0 _newtrack_1) (Timeline|Timeline_0_0 PlayFromStart)
    (:Update
      (Transformation|SetRelativeLocation _staticmesh (Math|Vector|MakeVector 0.0 0.0 (Math|Float|Lerp 3e+02 3e+01 _newtrack_0)) false false)
      (Transformation|SetWorldScale3D _staticmesh _newtrack_1))
    (:Finished
      (Actor|DestroyActor _gridpointref)
      (CallFunction|TraceSimple))
    (:NewTrack_2
      (Audio|PlaySoundatLocation "/Game/Sounds/Cues/DropCue.DropCue" (Transformation|GetWorldLocation _staticmesh) "0, 0, 0" 1.0 1.0 0.0 0 0 0))))

(fn ConstructionScript
  (|CallParentFunction))