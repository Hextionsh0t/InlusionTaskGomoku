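; Turn-based AI opponent that answers threats on a grid by spawning BP_PointEnemy on grid points.
; It registers itself with the player's BP_Character and relays the player's turn back to it.
; On AiTurn it checks four priority-ordered threat lists, matching each head index to a BP_GridPoint and consuming it on success.
; Without a match it spawns on a random grid point; the lists are filled outside this graph.
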(event Custom|AiTurn
  (CallFunction|CheckThreats))

(event Custom|initiatePlayerTurn
  (Default|PlayerTurn (Variables|Default|GetCharacterRef)))

(event Custom|CheckThreats
  (bind _veryhighthreats (Variables|Default|GetVeryHighThreats))
  (bind _highprioritythreats (Variables|Default|GetHighPriorityThreats))
  (bind _highthreats (Variables|Default|GetHighThreats))
  (bind _mediumthreats (Variables|Default|GetMediumThreats))
  (if (Utilities|Array|IsValidIndex _veryhighthreats)
    (bind _outactors (Actor|GetAllActorsOfClass "/Game/Blueprints/Bp_GridPoint.BP_GridPoint_C"))
    (Variables|Default|SetSucess? false)
    (for _array_element _outactors
      (if (== (Utilities|Array|Get(acopy) _veryhighthreats) (Variables|/Game/Blueprints/Bp_GridPoint.BP_GridPoint_C|GetGridPointIndex _array_element))
        (Variables|Default|SetTempPointRef _array_element)
        (Variables|Default|SetSucess? true)))
    (if (Variables|Default|GetSucess?)
      (Utilities|Array|RemoveIndex _veryhighthreats)
      (bind _asbp_grid_point (Utilities|Casting|CastToBP_GridPoint (Variables|Default|GetTempPointRef)))
      (Game|SpawnActorfromClass "/Game/Blueprints/BP_PointEnemy.BP_PointEnemy_C" (Math|Transform|MakeTransform (Transformation|GetActorLocation _asbp_grid_point) "0, 0, 0" "1,1,1") "AlwaysSpawn" 0 self 0)
      (else
        (if (Utilities|Array|IsValidIndex _highprioritythreats) :!label _label
          (bind _outactors_2 (Actor|GetAllActorsOfClass "/Game/Blueprints/Bp_GridPoint.BP_GridPoint_C"))
          (Variables|Default|SetSucess? false)
          (for _array_element_2 _outactors_2
            (if (== (Utilities|Array|Get(acopy) _highprioritythreats) (Variables|/Game/Blueprints/Bp_GridPoint.BP_GridPoint_C|GetGridPointIndex _array_element_2))
              (Variables|Default|SetTempPointRef _array_element_2)
              (Variables|Default|SetSucess? true)))
          (if (Variables|Default|GetSucess?)
            (Utilities|Array|RemoveIndex _highprioritythreats)
            (bind _asbp_grid_point_2 (Utilities|Casting|CastToBP_GridPoint (Variables|Default|GetTempPointRef)))
            (Game|SpawnActorfromClass "/Game/Blueprints/BP_PointEnemy.BP_PointEnemy_C" (Math|Transform|MakeTransform (Transformation|GetActorLocation _asbp_grid_point_2) "0, 0, 0" "1,1,1") "AlwaysSpawn" 0 self 0)
            (else
              (if (Utilities|Array|IsValidIndex _highthreats) :!label _label_2
                (bind _outactors_3 (Actor|GetAllActorsOfClass "/Game/Blueprints/Bp_GridPoint.BP_GridPoint_C"))
                (Variables|Default|SetSucess? false)
                (for _array_element_3 _outactors_3
                  (if (== (Utilities|Array|Get(acopy) _highthreats) (Variables|/Game/Blueprints/Bp_GridPoint.BP_GridPoint_C|GetGridPointIndex _array_element_3))
                    (Variables|Default|SetTempPointRef _array_element_3)
                    (Variables|Default|SetSucess? true)))
                (if (Variables|Default|GetSucess?)
                  (Utilities|Array|RemoveIndex _highthreats)
                  (bind _asbp_grid_point_3 (Utilities|Casting|CastToBP_GridPoint (Variables|Default|GetTempPointRef)))
                  (Game|SpawnActorfromClass "/Game/Blueprints/BP_PointEnemy.BP_PointEnemy_C" (Math|Transform|MakeTransform (Transformation|GetActorLocation _asbp_grid_point_3) "0, 0, 0" "1,1,1") "AlwaysSpawn" 0 self 0)
                  (else
                    (if (Utilities|Array|IsValidIndex _mediumthreats) :!label _label_3
                      (bind _outactors_4 (Actor|GetAllActorsOfClass "/Game/Blueprints/Bp_GridPoint.BP_GridPoint_C"))
                      (Variables|Default|SetSucess? false)
                      (for _array_element_4 _outactors_4
                        (if (== (Utilities|Array|Get(acopy) _mediumthreats) (Variables|/Game/Blueprints/Bp_GridPoint.BP_GridPoint_C|GetGridPointIndex _array_element_4))
                          (Variables|Default|SetTempPointRef _array_element_4)
                          (Variables|Default|SetSucess? true)))
                      (if (Variables|Default|GetSucess?)
                        (Utilities|Array|RemoveIndex _mediumthreats)
                        (bind _asbp_grid_point_4 (Utilities|Casting|CastToBP_GridPoint (Variables|Default|GetTempPointRef)))
                        (Game|SpawnActorfromClass "/Game/Blueprints/BP_PointEnemy.BP_PointEnemy_C" (Math|Transform|MakeTransform (Transformation|GetActorLocation _asbp_grid_point_4) "0, 0, 0" "1,1,1") "AlwaysSpawn" 0 self 0)
                        (else
                          (bind _outactors_5 (Actor|GetAllActorsOfClass "/Game/Blueprints/Bp_GridPoint.BP_GridPoint_C" :!label _label_4))
                          (bind _output_get (Variables|Default|SetRandomizedPointIndex (Math|Random|RandomIntegerinRange 0 (- (Utilities|Array|Length _outactors_5) 1))))
                          (Utilities|IsValid (Utilities|Array|Get(acopy) _outactors_5 _output_get)
                            (:Is%20Valid
                              (Variables|Default|SetTempIndex (Variables|/Game/Blueprints/Bp_GridPoint.BP_GridPoint_C|GetGridPointIndex (Utilities|Array|Get(acopy) _outactors_5 _output_get)))
                              (Game|SpawnActorfromClass "/Game/Blueprints/BP_PointEnemy.BP_PointEnemy_C" (Math|Transform|MakeTransform (Transformation|GetActorLocation (Utilities|Array|Get(acopy) _outactors_5 _output_get)) "0, 0, 0" "1,1,1") "AlwaysSpawn" 0 self 0)))))
                      (else
                        (goto _label_4)))))
                (else
                  (goto _label_3)))))
          (else
            (goto _label_2)))))
    (else
      (goto _label))))

(event EventBeginPlay
  (bind _asbp_character (Utilities|Casting|CastToBP_Character (Game|Player|GetPlayerPawn 0)))
  (bind _output_get (Variables|Default|SetCharacterRef _asbp_character))
  (Variables|/Game/Blueprints/BP_Character.BP_Character_C|SetMasterAIRef _output_get self))

(fn ConstructionScript)