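; Bp_GridPoint is a clickable grid point where the player makes a move on their turn.
; Clicking its Box during BP_Character's turn clears MyTurn, spawns a Bp_PointCharacterNEW at the root's location with references to the point and MasterAI, then calls CharacterMadeAMove.
; A DoOnce gate limits each point to one successful move, resetting only when the click happens out of turn.
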(event OnClicked(Box)
  (params (TouchedComponent :type Primitive%20Component%20Object%20Reference) (ButtonPressed :type Key%20Structure))
  (bind _asbp_character (Utilities|Casting|CastToBP_Character (Game|Player|GetPlayerPawn 0)))
  (Utilities|FlowControl|DoOnce false :!label _label
    (:Completed
      (if (Variables|/Game/Blueprints/BP_Character.BP_Character_C|GetMyTurn? _asbp_character)
        (Variables|/Game/Blueprints/BP_Character.BP_Character_C|SetMyTurn? _asbp_character false)
        (Game|SpawnActorfromClass "/Game/Blueprints/Bp_PointCharacterNEW.Bp_PointCharacterNEW_C" (Math|Transform|MakeTransform (Transformation|GetWorldLocation (Variables|Default|GetDefaultSceneRoot))) "AlwaysSpawn" 0 (Variables|Default|GetMasterAIref) self 0)
        (Default|CharacterMadeAMove _asbp_character)
        (else
          (goto _label Reset))))))

(fn ConstructionScript)